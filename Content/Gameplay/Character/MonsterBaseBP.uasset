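; Base Blueprint for monsters, providing the visual reaction when a sprite-based monster is hit.
; PlayHitAnim tints the sprite overbright red, sets the Struck status and runs a timeline that shakes it by random offsets scaled by an amplitude track.
; When the timeline finishes, the sprite's position and color reset and the status becomes Down at zero health, otherwise Idle.
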(event EventBeginPlay)

(event Collision|EventActorBeginOverlap
  (params (OtherActor :type Actor%20Object%20Reference)))

(event EventTick
  (params (DeltaSeconds :type Float%20%28single-precision%29)))

(event EventPlayHitAnim
  (params (bMajor :type Boolean))
  (bind _sprite (Variables|Default|GetSprite))
  (CallFunction|StartEndStruck true)
  (bind _amplitude (Timeline|HitTimeline PlayFromStart)
    (:Update
      (Transformation|SetRelativeLocation _sprite (* (* (Math|Random|RandomUnitVector) _amplitude) 1e+01) false false))
    (:Finished
      (CallFunction|StartEndStruck false)
      (Transformation|SetRelativeLocation _sprite "0, 0, 0" false false))))

(fn ConstructionScript)

(fn StartEndStruck
  (params (Start :type Boolean))
  (if Start
    (Class|GTCharacter|SetSpriteColor "(R=2.000000,G=0.000000,B=0.000000,A=1.000000)")
    (Variables|Default|SetStatusAnim "Struck")
    (else
      (Class|GTCharacter|SetSpriteColor "(R=1.000000,G=1.000000,B=1.000000,A=1.000000)")
      (Variables|Default|SetStatusAnim (select (== (Class|TargetableInterface|GetCurrentHealth) 0) "Down" "Idle")))))